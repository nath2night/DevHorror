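; BP_Knife is an interactable quest pickup that advances the objective chain when used, provided IsLastQuestDone is set.
; On Interact it destroys the BP_NpcInteract actor, increments the GI_Ressouce Index and updates the player's HUD objective flags before refreshing the objective.
; It then enables interaction on BP_Breaker, found by class lookup like the NPC, and destroys itself.
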(event `Interact`
  (if (`self.IsLastQuestDone?`)
    (bind _returnvalue (`GameplayStatics.GetActorOfClass` "/Game/Core/BP/BP_NpcInteract.BP_NpcInteract_C"))
    (`self.K2_DestroyActor` _returnvalue)
    (bind _asgi_ressouce (cast `/Game/Core/BP/GI_Ressouce` (`GameplayStatics.GetGameInstance`)))
    (`/Engine/EditorBlueprintResources/StandardMacros.IncrementInt` (`/Game/Core/BP/GI_Ressouce.Index` _asgi_ressouce)
      (:`  `
        (set `self.IsLastQuestDone?` false)
        (bind _asbp_first_person_character (cast `/Game/FirstPerson/Blueprints/BP_FirstPersonCharacter` (`GameplayStatics.GetPlayerPawn` 0)))
        (bind _widgethudref (`/Game/FirstPerson/Blueprints/BP_FirstPersonCharacter.WidgetHudRef` _asbp_first_person_character))
        (set `/Game/Core/Widget/WBP_Hud.Isdone2?` false _widgethudref)
        (set `/Game/Core/Widget/WBP_Hud.Isdone3?` true _widgethudref)
        (`/Game/Core/Widget/WBP_Hud.ChangeObjectif` _widgethudref)
        (bind _returnvalue_2 (`GameplayStatics.GetActorOfClass` "/Game/Core/BP/BP_Breaker.BP_Breaker_C"))
        (set `/Game/Core/BP/BP_Breaker.CanInteract?` true _returnvalue_2)
        (`self.K2_DestroyActor` self)))))

(fn `UserConstructionScript`)