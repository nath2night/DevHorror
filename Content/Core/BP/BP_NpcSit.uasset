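; BP_NpcSit is an NPC, seated by its name, with a separate mask that turns to follow the first-person player.
; On BeginPlay it caches the BP_FirstPersonCharacter player and hides the mesh's neck_01 bone, removing the body's own head.
; Each tick, MaskPivot smoothly interpolates toward the look-at rotation to the player, applying only world yaw so the mask stays level.
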(event `self.ReceiveBeginPlay`
  (bind _asbp_first_person_character (cast `/Game/FirstPerson/Blueprints/BP_FirstPersonCharacter` (`GameplayStatics.GetPlayerCharacter` 0)))
  (set `self.PlayerRef` _asbp_first_person_character)
  (`SkinnedMeshComponent.HideBoneByName` (`self.Mesh`) "neck_01" "PBO_None"))

(event `self.ReceiveTick`
  (params (DeltaSeconds :type "Float (single-precision)"))
  (bind _maskpivot (`self.MaskPivot`))
  (`/Engine/EditorBlueprintResources/StandardMacros.IsValid` (`self.PlayerRef`)
    (:`Is Valid`
      (`SceneComponent.K2_SetWorldRotation` (`self.MaskPivot`) (`KismetMathLibrary.MakeRotator` 0.0 0.0 (.yaw (`KismetMathLibrary.RInterpTo` (`SceneComponent.K2_GetComponentRotation` _maskpivot) (`KismetMathLibrary.FindLookAtRotation` (`SceneComponent.K2_GetComponentLocation` _maskpivot) (`self.K2_GetActorLocation` (`self.PlayerRef`))) DeltaSeconds 2.0))) false false))))

(fn `UserConstructionScript`)