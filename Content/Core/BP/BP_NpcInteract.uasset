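; Quest NPC Blueprint that the player can interact with once to advance the quest, with a floating arrow bobbing above it.
; Interact increments the GI_Ressouce game instance index, flips the HUD's done flags and refreshes the objective, then disables itself.
; It also marks the last quest done on the first BP_Knife in the level.
; A timeline started at BeginPlay animates the arrow's height over the actor.
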(event `Interact`
  ; ajouter le texte
  (if (`self.CanInteract?`)
    (bind _asgi_ressouce (cast `/Game/Core/BP/GI_Ressouce` (`GameplayStatics.GetGameInstance`)))
    (`/Engine/EditorBlueprintResources/StandardMacros.IncrementInt` (`/Game/Core/BP/GI_Ressouce.Index` _asgi_ressouce)
      (:`  `
        (bind _asbp_first_person_character (cast `/Game/FirstPerson/Blueprints/BP_FirstPersonCharacter` (`GameplayStatics.GetPlayerPawn` 0)))
        (bind _widgethudref (`/Game/FirstPerson/Blueprints/BP_FirstPersonCharacter.WidgetHudRef` _asbp_first_person_character))
        (set `/Game/Core/Widget/WBP_Hud.Isdone1?` false _widgethudref)
        (set `/Game/Core/Widget/WBP_Hud.Isdone2?` true _widgethudref)
        (`/Game/Core/Widget/WBP_Hud.ChangeObjectif` _widgethudref)
        (set `self.CanInteract?` false)
        (bind _returnvalue (`GameplayStatics.GetActorOfClass` "/Game/Core/BP/BP_Knife.BP_Knife_C"))
        (set `/Game/Core/BP/BP_Knife.IsLastQuestDone?` true _returnvalue)))))

(event `self.ReceiveBeginPlay`
  (bind (_direction _newtrack_0) (`Timeline|Timeline`)
    (:`Update`
      (`SceneComponent.K2_SetWorldLocation` (`self.ArrowQuest`) (`KismetMathLibrary.MakeVector` (.x (`self.K2_GetActorLocation`)) (.y (`self.K2_GetActorLocation`)) (+ _newtrack_0 (+ (.z (`self.K2_GetActorLocation`)) 150.0))) false false))))

(fn `UserConstructionScript`)