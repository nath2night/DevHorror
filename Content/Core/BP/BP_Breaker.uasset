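; BP_Breaker is an interactable breaker that shuts off the level's lights and advances the player's objective.
; On its first successful Interact, it loops over every BP_Light actor, setting its light intensity to zero.
; Inside that same loop it disables further interaction, increments the GI_Ressouce index once per light, updates the HUD objective flags and text, and enables the first-person character's attack.
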(event `Interact`
  (if (`self.CanInteract?`)
    (bind _outactors (`GameplayStatics.GetAllActorsOfClass` "/Game/Core/BP/BP_Light.BP_Light_C"))
    (if (> (`KismetArrayLibrary.Array_Length` _outactors) 0)
      (for (_ _array_index) _outactors
        (`LightComponent.SetIntensity` (`/Game/Core/BP/BP_Light.Light` (`|GetArrayItem` _outactors _array_index)) 0.0)
        (set `self.CanInteract?` false)
        (bind _asgi_ressouce (cast `/Game/Core/BP/GI_Ressouce` (`GameplayStatics.GetGameInstance`)))
        (`/Engine/EditorBlueprintResources/StandardMacros.IncrementInt` (`/Game/Core/BP/GI_Ressouce.Index` _asgi_ressouce)
          (:`  `
            (bind _asbp_first_person_character (cast `/Game/FirstPerson/Blueprints/BP_FirstPersonCharacter` (`GameplayStatics.GetPlayerPawn` 0)))
            (bind _widgethudref (`/Game/FirstPerson/Blueprints/BP_FirstPersonCharacter.WidgetHudRef` _asbp_first_person_character))
            (set `/Game/Core/Widget/WBP_Hud.Isdone3?` false _widgethudref)
            (set `/Game/Core/Widget/WBP_Hud.Isdone4?` true _widgethudref)
            (`/Game/Core/Widget/WBP_Hud.ChangeObjectif` _widgethudref)
            (set `/Game/FirstPerson/Blueprints/BP_FirstPersonCharacter.CanAttack?` true _asbp_first_person_character)))))))

(fn `UserConstructionScript`)