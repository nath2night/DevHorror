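; BP_VictimeController is the AI controller for the Victime character, making it react in fear when it sees the player.
; It runs BT_Victime on BeginPlay and listens to AI Perception updates for the first-person character.
; A successful sighting releases the pawn's hide point, stops movement, and updates the Blackboard to set the target, flag fear and request a new hide point.
; Losing perception of the player changes nothing here.
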(event `self.ReceiveBeginPlay`
  (`self.RunBehaviorTree` "/Game/Core/IA/BT_Victime.BT_Victime"))

(event `self.AIPerception.OnTargetPerceptionUpdated`
  (params (Actor :type "Actor Object Reference") (Stimulus :type "AIStimulus Structure"))
  (bind _returnvalue (`AIBlueprintHelperLibrary.GetBlackboard` null))
  (bind _asbp_first_person_character (cast `/Game/FirstPerson/Blueprints/BP_FirstPersonCharacter` Actor))
  (if (`.bSuccessfullySensed` (break `AIStimulus` Stimulus))
    (`KismetSystemLibrary.PrintString` "I see Player")
    (bind _asbp_victime (cast `/Game/Core/IA/BP_Victime` (`self.K2_GetPawn`)))
    (`/Game/Core/IA/BP_Victime.ReleaseCurrentHidePoint` _asbp_victime)
    (`self.StopMovement`)
    (`BlackboardComponent.SetValueAsObject` _returnvalue "CurrentHidePoint" null)
    (`BlackboardComponent.SetValueAsObject` _returnvalue "TargetActor" _asbp_first_person_character)
    (`BlackboardComponent.SetValueAsBool` _returnvalue "NeedNewHidePoint" true)
    (`BlackboardComponent.SetValueAsBool` _returnvalue "IsScared" true)))

(fn `UserConstructionScript`)