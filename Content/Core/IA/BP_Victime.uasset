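; BP_Victime is an AI-driven victim that flees to hide points and reacts when the first-person player damages it.
; On player damage it frees its current BP_HidePoint by clearing occupancy and the blackboard key, and stops controller movement.
; It then sets the attacker as TargetActor and raises IsScared and NeedNewHidePoint in the blackboard, leaving the response to the AI logic.
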(event `self.ReceiveAnyDamage`
  (params (Damage :type "Float (single-precision)") (DamageType :type "DamageType Object Reference") (InstigatedBy :type "Controller Object Reference") (DamageCauser :type "Actor Object Reference"))
  (bind _returnvalue (`self.GetController`))
  (bind _returnvalue_2 (`AIBlueprintHelperLibrary.GetBlackboard` _returnvalue))
  (bind _asbp_first_person_character (cast `/Game/FirstPerson/Blueprints/BP_FirstPersonCharacter` DamageCauser))
  (`KismetSystemLibrary.PrintString` "im hit")
  (`self.ReleaseCurrentHidePoint`)
  (`Controller.StopMovement` (cast `/Game/Core/IA/BP_VictimeController` _returnvalue :!pure true))
  (`BlackboardComponent.SetValueAsObject` _returnvalue_2 "CurrentHidePoint" null)
  (`BlackboardComponent.SetValueAsObject` _returnvalue_2 "TargetActor" _asbp_first_person_character)
  (`BlackboardComponent.SetValueAsBool` _returnvalue_2 "NeedNewHidePoint" true)
  (`BlackboardComponent.SetValueAsBool` _returnvalue_2 "IsScared" true))

(fn `ReleaseCurrentHidePoint`
  (bind _asbp_victime_controller (cast `/Game/Core/IA/BP_VictimeController` (`self.GetController`)))
  (bind _returnvalue (`AIBlueprintHelperLibrary.GetBlackboard` _asbp_victime_controller))
  (bind _returnvalue_2 (`BlackboardComponent.GetValueAsObject` _returnvalue "CurrentHidePoint"))
  (if (`KismetSystemLibrary.IsValid` _returnvalue_2)
    (bind _asbp_hide_point (cast `/Game/Core/IA/BP_HidePoint` _returnvalue_2))
    (set `/Game/Core/IA/BP_HidePoint.IsOccupied` false _asbp_hide_point)
    (set `/Game/Core/IA/BP_HidePoint.OccupyingAi` null _asbp_hide_point)
    (`BlackboardComponent.SetValueAsObject` _returnvalue "CurrentHidePoint" null)))

(fn `UserConstructionScript`)